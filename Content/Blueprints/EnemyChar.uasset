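; Enemy character Blueprint that patrols a looping route of waypoint actors through its AI controller.
; BeginPlay starts an AI MoveTo toward the current entry in the Waypoints array.
; When each move finishes, the index advances with modulo wraparound and the WaypointReached event fires to start the next move, so the patrol repeats without using Tick.
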(event Custom|Event%20WaypointReached
  ;[1 1 1] Move through waypoints
  (AI|AIMoveTo (AI|GetAIController self) "0, 0, 0" (Utilities|Array|Get(acopy) (Variables|Default|GetWaypoints) (Variables|Default|GetWaypoint%20to%20reference)) -1.0 "Default" "Default" true true
    (:OnMoveFinished
      (Variables|Default|SetWaypoint%20to%20reference (Math|Integer|%(Integer) (+ (Variables|Default|GetWaypoint%20to%20reference) 1) (Utilities|Array|Length (Variables|Default|GetWaypoints))))
      (CallFunction|EventWaypointReached))))

(event EventBeginPlay
  ;[1 1 1] Move through waypoints
  (AI|AIMoveTo (AI|GetAIController self) "0, 0, 0" (Utilities|Array|Get(acopy) (Variables|Default|GetWaypoints) (Variables|Default|GetWaypoint%20to%20reference)) -1.0 "Default" "Default" true true
    (:OnMoveFinished
      (Variables|Default|SetWaypoint%20to%20reference (Math|Integer|%(Integer) (+ (Variables|Default|GetWaypoint%20to%20reference) 1) (Utilities|Array|Length (Variables|Default|GetWaypoints))))
      (CallFunction|EventWaypointReached))))

(fn ConstructionScript)