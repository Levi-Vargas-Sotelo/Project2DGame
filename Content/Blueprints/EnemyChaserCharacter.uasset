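; Enemy chaser character that relays AI Perception results to its AIC_2Dcharacter controller, maintaining the line-of-sight and target actor keys.
; A successful sense cancels any pending target-lost timer and passes the perceived actor to the controller as the target.
; A lost sense clears line of sight at once but starts a short grace timer, after which the target is cleared.
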(event OnTargetPerceptionUpdated(AIPerception)
  (params (Actor :type Actor%20Object%20Reference) (Stimulus :type AI%20Stimulus%20Structure))
  (Variables|Default|SetPerceived%20Actor Actor)
  (if (.bSuccessfullySensed (Utilities|Struct|BreakAIStimulus Stimulus))
    (Utilities|Time|ClearandInvalidateTimerbyHandle (Variables|Default|GetTargetLostTimer))
    (Default|UpdateLineOfSightKey (.AsAIC%202Dcharacter (Utilities|Casting|CastToAIC_2Dcharacter (Pawn|GetController))) true)
    (Default|TargetActorKey (.AsAIC%202Dcharacter (Utilities|Casting|CastToAIC_2Dcharacter (Pawn|GetController))) (Variables|Default|GetPerceived%20Actor))
    (else
      (bind _returnvalue (Utilities|Time|SetTimerbyEvent (delegate Custom|On%20Target%20Lost) 2.5))
      (Variables|Default|SetTargetLostTimer _returnvalue)
      (Default|UpdateLineOfSightKey (.AsAIC%202Dcharacter (Utilities|Casting|CastToAIC_2Dcharacter (Pawn|GetController))) false))))

(event Custom|On%20Target%20Lost
  (Variables|Default|SetPerceived%20Actor 0)
  (Default|TargetActorKey (.AsAIC%202Dcharacter (Utilities|Casting|CastToAIC_2Dcharacter (Pawn|GetController)))))

(fn ConstructionScript)